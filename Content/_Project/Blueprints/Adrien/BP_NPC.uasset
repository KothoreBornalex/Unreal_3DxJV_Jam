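; Enemy NPC that signals its presence to nearby players and sends the player back to their start position on contact.
; A looping timer plays a radial presence camera shake around the NPC every second.
; A capsule hit on the player character freezes both, blends the view to the NPC and plays a catch shake.
; After a short delay it teleports the player, resets control rotation and restores movement and view.
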(event OnComponentHit(CapsuleComponent)
  (params (HitComponent :type Primitive%20Component%20Object%20Reference) (OtherActor :type Actor%20Object%20Reference) (OtherComp :type Primitive%20Component%20Object%20Reference) (NormalImpulse :type Vector :default "0, 0, 0") (Hit :type Hit%20Result%20Structure%20%28by%20ref%29))
  (bind _returnvalue (Game|GetPlayerController 0))
  (bind _asbp_character_framework (Utilities|Casting|CastToBP_Character_Framework OtherActor))
  (Variables|Default|SetAs%20BP%20Character%20Framework _asbp_character_framework)
  (Pawn|Components|CharacterMovement|DisableMovement (Variables|Character|GetCharacterMovement))
  (Pawn|Components|CharacterMovement|DisableMovement (Variables|/Script/Engine.Character|GetCharacterMovement (Variables|Default|GetAs%20BP%20Character%20Framework)))
  (Game|Player|SetViewTargetwithBlend (Game|GetPlayerController 0) self 0.25 "VTBlend_EaseIn" 0.3 false)
  (Camera|PlayWorldCameraShake "/Game/_Project/Blueprints/Adrien/Headshake/BP_CatchCamShake.BP_CatchCamShake_C" (Transformation|GetActorLocation) 0.0 1e+03)
  (Utilities|FlowControl|Delay 1.0)
  (Transformation|Teleport (Variables|Default|GetAs%20BP%20Character%20Framework) (Variables|/Game/_Project/Blueprints/Ibrahim/Core/BP_Character_Framework.BP_Character_Framework_C|GetStartPos (Variables|Default|GetAs%20BP%20Character%20Framework)) "0, 0, 0")
  (Pawn|SetControlRotation _returnvalue (Math|Rotator|MakeRotator 0.0 0.0 0.0))
  (Pawn|Components|CharacterMovement|SetMovementMode (Variables|/Script/Engine.Character|GetCharacterMovement (Variables|Default|GetAs%20BP%20Character%20Framework)) "MOVE_Walking" 0)
  (Game|Player|SetViewTargetwithBlend _returnvalue (Variables|Default|GetAs%20BP%20Character%20Framework) 0.0 "VTBlend_Linear" 0.0 false)
  (Pawn|Components|CharacterMovement|SetMovementMode (Variables|Character|GetCharacterMovement) "MOVE_Walking" 0))

(event Custom|HeadShakePresence
  (Camera|PlayWorldCameraShake "/Game/_Project/Blueprints/Adrien/Headshake/BP_IAPresenceHS.BP_IAPresenceHS_C" (Transformation|GetActorLocation) 0.0 1e+03))

(event EventBeginPlay
  (Variables|Default|SetWalk%20Speed (Variables|/Script/Engine.CharacterMovementComponent|GetMaxWalkSpeed (Variables|Character|GetCharacterMovement)))
  (Utilities|Time|SetTimerbyEvent (delegate Custom|HeadShakePresence) 1.0 true))

(fn ConstructionScript)