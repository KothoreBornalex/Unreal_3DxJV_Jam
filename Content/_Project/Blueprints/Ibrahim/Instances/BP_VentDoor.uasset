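; BP_VentDoor is an interactable vent door that slides sideways open once, playing an opening sound on each Interact call.
; It stores the mesh's starting location at BeginPlay, and IsLeftSide picks the mesh's left or right vector as the slide direction.
; A timeline lerps the mesh from its current location toward the offset target, while a Used flag blocks reopening.
; IsInteractible always returns false.
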(event Custom|OpenVentDoor
  (if (not (Variables|Default|GetUsed))
    (Variables|Default|SetUsed true)
    (if (Variables|Default|GetIsLeftSide)
      (Variables|Default|SetDirVector (* (Math|Vector|GetRightVector (Variables|Default|GetDoorVentMesh)) -1.0))
      (bind _dooranimation (Timeline|TL_DoorAnimation PlayFromStart)
        (:Update
          (Transformation|SetWorldLocation (Variables|Default|GetDoorVentMesh) (Math|Vector|Lerp(Vector) (Transformation|GetWorldLocation (Variables|Default|GetDoorVentMesh)) (+ (Variables|Default|GetBaseLocation) (* (Variables|Default|GetDirVector) (Variables|Default|GetDoorOffset))) _dooranimation) false false)))
      (else
        (Variables|Default|SetDirVector (Math|Vector|GetRightVector (Variables|Default|GetDoorVentMesh)))
        (Timeline|TL_DoorAnimation PlayFromStart)))))

(event EventBeginPlay
  (Variables|Default|SetBaseLocation (Transformation|GetWorldLocation (Variables|Default|GetDoorVentMesh))))

(event EventTick
  (params (DeltaSeconds :type Float%20%28single-precision%29)))

(event EventInteract
  (params (RequestOwner :type Pawn%20Object%20Reference))
  (CallFunction|OpenVentDoor)
  (Audio|PlaySoundatLocation "/Game/SoundDesign/OPENING_VENT.OPENING_VENT" (Transformation|GetActorLocation) "0, 0, 0" 1.0 1.0 0.0 0 0 0 0))

(fn ConstructionScript)

(fn IsInteractible
  (return false))