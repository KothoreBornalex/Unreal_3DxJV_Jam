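; BP_CrownFragment is a crown fragment pickup that emits a looping or ambient positional sound from BeginPlay.
; Interact adds a fragment to the requester's AC_Helmet component, plays a pickup sound and starts removal, although IsInteractible returns false.
; Removal stops the ambient sound, reports an AI noise event, hides the box hierarchy and disables mesh collision, leaving the actor undestroyed.
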(event Custom|StartDestroy
  (Audio|Components|Audio|Stop (Variables|Default|GetEmanentSound))
  (Class|AISenseHearing|ReportNoiseEvent (Transformation|GetActorLocation) 1.0 self 1e+03 "None")
  (Rendering|SetVisibility (Variables|Default|GetBox) false true)
  (Collision|SetCollisionEnabled (Variables|Default|GetStaticMesh) "NoCollision"))

(event EventBeginPlay
  (bind _returnvalue (Audio|SpawnSoundatLocation "/Game/SoundDesign/EMANENT_OBJECT.EMANENT_OBJECT" (Transformation|GetActorLocation) "0, 0, 0" 1.0 1.0 0.0 "/Game/SoundDesign/SA_EMANENT_OBJECT.SA_EMANENT_OBJECT" 0))
  (Variables|Default|SetEmanentSound _returnvalue))

(event EventInteract
  (params (RequestOwner :type Pawn%20Object%20Reference))
  (bind _returnvalue (Actor|GetComponentbyClass RequestOwner "/Game/_Project/Blueprints/Ibrahim/Systems/HelmetSystem/AC_Helmet.AC_Helmet_C"))
  (Utilities|IsValid _returnvalue
    (:Is%20Valid
      (Default|AddFragment _returnvalue)
      (Audio|PlaySoundatLocation "/Engine/VREditor/Sounds/UI/Object_PickUp.Object_PickUp" (Transformation|GetActorLocation) "0, 0, 0" 1.0 1.0 0.0 "/Game/SoundDesign/SA_EMANENT_OBJECT.SA_EMANENT_OBJECT" 0 0 0)
      (CallFunction|StartDestroy))))

(fn ConstructionScript)

(fn IsInteractible
  (return false))