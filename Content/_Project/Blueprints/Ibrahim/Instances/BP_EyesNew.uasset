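; BP_EyesNew is a non-interactible eyes actor that slowly turns to follow the player.
; After a short delay on BeginPlay it caches the pawn controlled by the first player controller.
; Each Tick it smoothly interpolates its rotation toward a look-at rotation aimed at that pawn, using RInterpTo.
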(event EventBeginPlay
  (Utilities|FlowControl|Delay 0.12)
  (Variables|Default|SetPlayerPawn (Pawn|GetControlledPawn (Game|GetPlayerController 0))))

(event EventTick
  (params (DeltaSeconds :type Float%20%28single-precision%29))
  (Utilities|IsValid (Variables|Default|GetPlayerPawn)
    (:Is%20Valid
      (Transformation|SetActorRotation (Math|Interpolation|RInterpTo (Transformation|GetActorRotation) (Math|Rotator|FindLookatRotation (Transformation|GetActorLocation) (Transformation|GetActorLocation (Variables|Default|GetPlayerPawn))) (Utilities|Time|GetWorldDeltaSeconds) 2.0)))))

(fn ConstructionScript)

(fn IsInteractible
  (return false))