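; BP_CrownHelmet is a crown helmet fragment pickup that plays an emanating sound from BeginPlay.
; Interact adds a fragment to the requester's AC_Helmet component, plays a grab sound and calls StartDestroy.
; If the emanating sound is valid, StartDestroy stops it, reports AI noise, hides Box and its children, and disables collision.
; The actor is never destroyed, and IsInteractible always returns false.
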(event Custom|StartDestroy
  (bind _emanentsound (Variables|Default|GetEmanentSound))
  (Utilities|IsValid _emanentsound
    (:Is%20Valid
      (Audio|Components|Audio|Stop _emanentsound)
      (Class|AISenseHearing|ReportNoiseEvent (Transformation|GetActorLocation) 1.0 self 1e+03 "None")
      (Rendering|SetVisibility (Variables|Default|GetBox) false true)
      (Collision|SetCollisionEnabled (Variables|Default|GetStaticMesh) "NoCollision"))))

(event EventBeginPlay
  (bind _returnvalue (Audio|SpawnSoundatLocation "/Game/SoundDesign/EMANENT_OBJECT.EMANENT_OBJECT" (Transformation|GetActorLocation) "0, 0, 0" 1.0 1.0 0.0 "/Game/SoundDesign/SA_EMANENT_OBJECT.SA_EMANENT_OBJECT" 0))
  (Variables|Default|SetEmanentSound _returnvalue))

(event EventInteract
  (params (RequestOwner :type Pawn%20Object%20Reference))
  (bind _returnvalue (Actor|GetComponentbyClass RequestOwner "/Game/_Project/Blueprints/Ibrahim/Systems/HelmetSystem/AC_Helmet.AC_Helmet_C"))
  (Utilities|IsValid _returnvalue
    (:Is%20Valid
      (Default|AddFragment _returnvalue)
      (Audio|PlaySoundatLocation "/Game/SoundDesign/GRAB_HELLMET.GRAB_HELLMET" (Transformation|GetActorLocation) "0, 0, 0" 1.0 1.0 0.0 "/Game/SoundDesign/SA_EMANENT_OBJECT.SA_EMANENT_OBJECT" 0 0 0)
      (CallFunction|StartDestroy))))

(fn ConstructionScript)

(fn IsInteractible
  (return false))