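; Player controller for the framework that sets up input, requests its spawn from the game mode and signals the pause menu.
; BeginPlay adds the movement, weapon and action Enhanced Input mapping contexts, then after a short delay passes itself to Spawn on BP_GM_Framework.
; It also sets game-only input mode in a parallel sequence branch.
; The pause input fires the EDPauseMenu event dispatcher, leaving the menu handling to its listeners.
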(event Input|EnhancedActionEvents|EnhancedInputActionIA_PauseMenu
  (params (ActionValue :type Boolean) (ElapsedSeconds :type Float%20%28double-precision%29) (TriggeredSeconds :type Float%20%28double-precision%29) (InputAction :type Input%20Action%20Object%20Reference :default "/Game/_Project/Inputs/Actions/IA_PauseMenu.IA_PauseMenu"))
  ;[0.4206 0.9435 1 1 66] PAUSE MENU
  (:Started
    (Default|CallEDPauseMenu)))

(event EventBeginPlay
  (bind _returnvalue (PlayerController|LocalPlayerSubsystems|GetEnhancedInputLocalPlayerSubsystem))
  (Utilities|FlowControl|Sequence
    (:then_0
      (Input|AddMappingContext _returnvalue "/Game/_Project/Inputs/IMC_Movements.IMC_Movements" 0 "(bIgnoreAllPressedKeysUntilRelease=True,bForceImmediately=False,bNotifyUserSettings=False)")
      (Input|AddMappingContext _returnvalue "/Game/FirstPerson/Input/IMC_Weapons.IMC_Weapons" 0 "(bIgnoreAllPressedKeysUntilRelease=True,bForceImmediately=False,bNotifyUserSettings=False)")
      (Input|AddMappingContext _returnvalue "/Game/_Project/Inputs/IMC_Actions.IMC_Actions" 0 "(bIgnoreAllPressedKeysUntilRelease=True,bForceImmediately=False,bNotifyUserSettings=False)")
      (Utilities|FlowControl|Delay 0.1)
      (bind _asbp_gm_framework (Utilities|Casting|CastToBP_GM_Framework (Game|GetGameMode)))
      (Development|PrintString "Hello")
      (Default|Spawn _asbp_gm_framework self))
    (:then_1
      (Input|SetInputModeGameOnly self false))))

(fn ConstructionScript)