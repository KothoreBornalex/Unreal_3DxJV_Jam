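; HUD framework that creates and drives the player's gameplay HUD and options-based pause menu.
; Player controller and menu dispatchers feed menu handling, with a FlipFlop switching visibility, input mode and cursor without pausing the game.
; On possessed pawn change, it binds character and helmet component events to update the interact prompt and fragment display.
; Victory and quit-to-menu fade the screen before loading MainMenuLevel, using a fade-finished event and a fixed delay respectively.
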(event Custom|Create%20HUD
  (bind _returnvalue (UserInterface|CreateWidget "/Game/_Project/Blueprints/Ibrahim/UI/HUD/WBP_HUD.WBP_HUD_C"))
  (Variables|Default|SetWBP_HUD _returnvalue)
  (UserInterface|Viewport|AddtoViewport _returnvalue 0)
  (Default|ActivateTips (Variables|Default|GetWBP_HUD)))

(event Custom|BaseSetUp
  (Pawn|BindEventtoOnPossessedPawnChanged (Variables|Default|GetPlayerOwner) (EventDispatchers|CreateEvent :!event Custom|OnPawnChanged))
  (bind _asbp_pc_framework (Utilities|Casting|CastToBP_PC_Framework (Variables|Default|GetPlayerOwner)))
  (EventDispatchers|BindEventtoEDPauseMenu _asbp_pc_framework (EventDispatchers|CreateEvent :!event Custom|TriggerPauseMenu)))

(event Custom|BackToMainMenu
  (Default|StartFadein (Variables|/Game/_Project/Blueprints/Ibrahim/UI/HUD/WBP_HUD.WBP_HUD_C|GetFadeInOut (Variables|Default|GetWBP_HUD)))
  (Utilities|FlowControl|Delay 4.0)
  (Game|OpenLevel(byName) "MainMenuLevel"))

(event Custom|OnPawnChanged
  (params (OldPawn :type Pawn%20Object%20Reference) (NewPawn :type Pawn%20Object%20Reference))
  ;[0.1615 0.1615 0.1615 1 110] ON PLAYER PAWN CHANGED
  (Utilities|IsValid NewPawn
    (:Is%20Valid
      (bind _asbp_character_framework (Utilities|Casting|CastToBP_Character_Framework NewPawn))
      (bind _output_get (Variables|Default|SetPlayerPawn _asbp_character_framework))
      (EventDispatchers|BindEventtoEDInteractibleEnterView _output_get (delegate Custom|OnInteractibleEnterView))
      (EventDispatchers|BindEventtoEDExitView (Variables|Default|GetPlayerPawn) (delegate Custom|OnInteractibleExitView))
      (EventDispatchers|BindEventtoEDVictoryEndGame (Variables|Default|GetPlayerPawn) (delegate Custom|OnVictoryEndGame))
      (EventDispatchers|BindEventtoEDFragmentUpdate (Actor|GetComponentbyClass (Variables|Default|GetPlayerPawn) "/Game/_Project/Blueprints/Ibrahim/Systems/HelmetSystem/AC_Helmet.AC_Helmet_C") (delegate Custom|OnFragmentUpdated)))))

(event Custom|OnVictoryEndGame
  (bind _wbp_hud (Variables|Default|GetWBP_HUD))
  (bind _fadeinout (Variables|/Game/_Project/Blueprints/Ibrahim/UI/HUD/WBP_HUD.WBP_HUD_C|GetFadeInOut _wbp_hud))
  ;[0.1615 0.1615 0.1615 1 110] ON PLAYER PAWN CHANGED
  (Default|StartFadein _fadeinout)
  (EventDispatchers|BindEventtoEDFadeinFinished _fadeinout (delegate Custom|OnVictory_FadeInFinished)))

(event Custom|OnInteractibleEnterView
  ;[0.1615 0.1615 0.1615 1 110] ON PLAYER PAWN CHANGED
  (Default|ActivateInteract (Variables|Default|GetWBP_HUD)))

(event Custom|OnInteractibleExitView
  ;[0.1615 0.1615 0.1615 1 110] ON PLAYER PAWN CHANGED
  (Default|DesactivateInteract (Variables|Default|GetWBP_HUD)))

(event Custom|OnVictory_FadeInFinished
  ;[0.1615 0.1615 0.1615 1 110] ON PLAYER PAWN CHANGED
  (Game|OpenLevel(byName) "MainMenuLevel"))

(event Custom|Create_PauseMenu
  (bind _returnvalue (UserInterface|CreateWidget "/Game/_Project/Blueprints/Adrien/Widget/W_Options.W_Options_C"))
  (bind _output_get (Variables|Default|SetWBP_PauseMenu _returnvalue))
  (UserInterface|Viewport|AddtoViewport _output_get 0)
  (Widget|SetVisibility _output_get "Collapsed")
  (EventDispatchers|BindEventtoEDClose _output_get (EventDispatchers|CreateEvent :!event Custom|TriggerPauseMenu))
  (EventDispatchers|BindEventtoEDGoBacktoMainMenu (Variables|Default|GetWBP_PauseMenu) (EventDispatchers|CreateEvent :!event Custom|BackToMainMenu)))

(event Custom|TriggerPauseMenu
  (bind _wbp_pausemenu (Variables|Default|GetWBP_PauseMenu))
  (bind _playerowner (Variables|Default|GetPlayerOwner))
  (bind _playerowner_2 (Variables|Default|GetPlayerOwner))
  (Utilities|FlowControl|FlipFlop
    (:A
      (Widget|SetVisibility _wbp_pausemenu "Visible")
      (Input|SetInputModeUIOnly _playerowner_2 0 "DoNotLock" false)
      (Variables|/Script/Engine.PlayerController|SetbShowMouseCursor _playerowner true))
    (:B
      (Widget|SetVisibility _wbp_pausemenu "Collapsed")
      (Input|SetInputModeGameOnly _playerowner_2 false)
      (Variables|/Script/Engine.PlayerController|SetbShowMouseCursor _playerowner false))))

(event Custom|OnFragmentUpdated
  (params (Fragment :type Integer))
  (bind _wbp_hud (Variables|Default|GetWBP_HUD))
  ;[0.1615 0.1615 0.1615 1 110] ON PLAYER PAWN CHANGED
  (switch int Fragment
    (:Default
      (Default|UpdateFragments _wbp_hud Fragment))
    (:1
      (Default|ActiveFragmentsInterface _wbp_hud true))))

(event EventBeginPlay
  (CallFunction|BaseSetUp)
  (CallFunction|CreatePauseMenu)
  (CallFunction|CreateHUD))

(fn ConstructionScript)