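; AC_Helmet is a component that counts collected helmet fragments and ties that progress to door activation in the map.
; On BeginPlay it caches the BP_MapManager actor found in the level.
; AddFragment increments the count, calls UpdateDoors and prints the total.
; UpdateDoors passes the count to the map manager's ActivateDoor, then broadcasts it through the EDFragmentUpdate dispatcher.
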(event Custom|UpdateDoors
  (bind _fragments (Variables|Default|GetFragments))
  (Default|ActivateDoor (Variables|Default|GetMapManager) _fragments)
  (Default|CallEDFragmentUpdate _fragments))

(event Custom|AddFragment
  (bind _output_get (Variables|Default|SetFragments (+ (Variables|Default|GetFragments) 1)))
  (CallFunction|UpdateDoors)
  (Development|PrintString (Utilities|String|ToString(Integer) _output_get)))

(event EventBeginPlay
  (bind _returnvalue (Actor|GetActorOfClass "/Game/_Project/Blueprints/Ibrahim/Systems/MapSystem/BP_MapManager.BP_MapManager_C"))
  (Variables|Default|SetMapManager _returnvalue))

(event EventTick
  (params (DeltaSeconds :type Float%20%28single-precision%29)))